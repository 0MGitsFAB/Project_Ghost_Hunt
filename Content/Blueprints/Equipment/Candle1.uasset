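; Candle equipment actor that the player can pick up, hold and throw when dropped.
; Pick Up disables physics on the candle holder and attaches it to the first-person character's item hold point, zeroing its relative rotation.
; Drop detaches it, restores physics, unhides the actor and applies an impulse along its Forward vector.
; GetIsHeld always returns false, so held state is not tracked here.
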(event EventDrop
  ;[1 1 1] Drop
  (Transformation|DetachFromActor "KeepWorld" "KeepRelative" "KeepWorld")
  (Physics|SetSimulatePhysics (Variables|Default|GetCandleHolder) true)
  (Rendering|SetActorHiddenInGame false)
  (Physics|AddImpulse (Variables|Default|GetCandleHolder) (* (Math|Vector|GetForwardVector (Variables|Default|GetForward)) 1e+03) "None" false))

(event EventPickUp
  (bind _candleholder (Variables|Default|GetCandleHolder))
  ;[1 1 1] Pick Up
  (Physics|SetSimulatePhysics _candleholder false) ; Disable Physics so it can sit in a single point in the world
  (bind _asbp_first_person_character (Utilities|Casting|CastToBP_FirstPersonCharacter (Game|GetPlayerCharacter 0)))
  (Transformation|AttachComponentToComponent _candleholder (Variables|/Game/Blueprints/Character/BP_FirstPersonCharacter.BP_FirstPersonCharacter_C|GetItemHoldPoint _asbp_first_person_character) "None" "KeepRelative" "KeepRelative" "KeepWorld" true) ; Make the Torch a child of the Item Hold Point
  (Transformation|SetWorldLocation _candleholder (Transformation|GetWorldLocation (Variables|/Game/Blueprints/Character/BP_FirstPersonCharacter.BP_FirstPersonCharacter_C|GetItemHoldPoint _asbp_first_person_character)) false false) ; Set the World Location of the Torch to the World Location of the Item Hold Point
  (Transformation|SetRelativeRotation _candleholder "0,0.000000, 0" false false) ; Set the Relative Rotation so it sits nicely in hand
)

(fn ConstructionScript)

(fn GetIsHeld
  (return false))