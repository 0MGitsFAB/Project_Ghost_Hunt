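; BP_MotionSensor is a motion sensor equipment item the first-person player can pick up, carry and drop.
; PickUp disables physics on the Body, attaches it to the character's ItemHoldPoint and rotates it to sit in hand.
; Drop detaches it, restores physics and visibility, and throws it with an impulse along its Forward component.
; The Use event is empty, so no sensing behavior is implemented here.
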(event EventUse)

(event EventDrop
  ;[1 1 1] Drop
  (Transformation|DetachFromActor "KeepWorld" "KeepRelative" "KeepWorld")
  (Physics|SetSimulatePhysics (Variables|Default|GetBody) true)
  (Rendering|SetActorHiddenInGame false)
  (Physics|AddImpulse (Variables|Default|GetBody) (* (Math|Vector|GetForwardVector (Variables|Default|GetForward)) 1e+03) "None" false))

(event EventPickUp
  (bind _body (Variables|Default|GetBody))
  ;[1 1 1] Pick Up
  (Physics|SetSimulatePhysics _body false) ; Disable Physics so it can sit in a single point in the world
  (bind _asbp_first_person_character (Utilities|Casting|CastToBP_FirstPersonCharacter (Game|GetPlayerCharacter 0)))
  (Transformation|AttachComponentToComponent _body (Variables|/Game/Blueprints/Character/BP_FirstPersonCharacter.BP_FirstPersonCharacter_C|GetItemHoldPoint _asbp_first_person_character) "None" "KeepRelative" "KeepRelative" "KeepWorld" true) ; Make the Torch a child of the Item Hold Point
  (Transformation|SetWorldLocation _body (Transformation|GetWorldLocation (Variables|/Game/Blueprints/Character/BP_FirstPersonCharacter.BP_FirstPersonCharacter_C|GetItemHoldPoint _asbp_first_person_character)) false false) ; Set the World Location of the Torch to the World Location of the Item Hold Point
  (Transformation|SetRelativeRotation _body "0,90.000000,90.000000" false false) ; Set the Relative Rotation so it sits nicely in hand
)

(fn ConstructionScript)