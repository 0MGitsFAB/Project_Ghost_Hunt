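; Handheld EMF reader that can be picked up, dropped with a forward impulse and switched on or off while held.
; Pick Up attaches its body to the player's ItemHoldPoint; Use toggles power and the first light.
; While on, overlaps with BP_InteractionEmitter actors pass their EMFLevel to ChangeState, which lights up to five lights by material swaps.
; ResetState clears the upper lights on power-off or overlap end, then remaining emitters are re-read.
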(event OnComponentBeginOverlap(Body)
  (params (OverlappedComponent :type Primitive%20Component%20Object%20Reference) (OtherActor :type Actor%20Object%20Reference) (OtherComp :type Primitive%20Component%20Object%20Reference) (OtherBodyIndex :type Integer) (bFromSweep :type Boolean) (SweepResult :type Hit%20Result%20Structure%20%28by%20ref%29))
  (bind _asinteraction_emitter (Utilities|Casting|CastToBP_InteractionEmitter OtherActor))
  (if (Variables|Default|GetIsOn)
    (CallFunction|ChangeState (Variables|/Game/Blueprints/Equipment/EMF/BP_InteractionEmitter.BP_InteractionEmitter_C|GetEMFLevel _asinteraction_emitter))))

(event OnComponentEndOverlap(Body)
  (params (OverlappedComponent :type Primitive%20Component%20Object%20Reference) (OtherActor :type Actor%20Object%20Reference) (OtherComp :type Primitive%20Component%20Object%20Reference) (OtherBodyIndex :type Integer))
  (bind _body (Variables|Default|GetBody))
  (bind _overlappingactors (Collision|GetOverlappingActors _body "/Game/Blueprints/Equipment/EMF/BP_InteractionEmitter.BP_InteractionEmitter_C" :!class /Script/Engine.PrimitiveComponent))
  (Utilities|Casting|CastToBP_InteractionEmitter OtherActor)
  (if (Utilities|Array|IsEmpty _overlappingactors)
    (CallFunction|ResetState)
    (else
      (for _array_element _overlappingactors
        (bind _asinteraction_emitter (Utilities|Casting|CastToBP_InteractionEmitter _array_element))
        (CallFunction|ResetState)
        (CallFunction|ChangeState (Variables|/Game/Blueprints/Equipment/EMF/BP_InteractionEmitter.BP_InteractionEmitter_C|GetEMFLevel _asinteraction_emitter))))))

(event EventUse
  (bind _light1 (Variables|Default|GetLight1))
  ;[1 1 1] Interact
  (if (Variables|Default|GetIsHeld)
    (bind _output_get (Variables|Default|SetIsOn (not (Variables|Default|GetIsOn))))
    (if _output_get
      (Rendering|Material|SetMaterial _light1 0 "/Game/Models/EMF/Material_001.Material_001")
      (bind _array_element (Utilities|Array|ForEachLoopwithBreak (Collision|GetOverlappingActors (Variables|Default|GetBody) "/Game/Blueprints/Equipment/EMF/BP_InteractionEmitter.BP_InteractionEmitter_C" :!class /Script/Engine.PrimitiveComponent) :!label _label)
        (:LoopBody
          (bind _asinteraction_emitter (Utilities|Casting|CastToBP_InteractionEmitter _array_element))
          (CallFunction|ChangeState (Variables|/Game/Blueprints/Equipment/EMF/BP_InteractionEmitter.BP_InteractionEmitter_C|GetEMFLevel _asinteraction_emitter))
          (goto _label Break)))
      (else
        (Rendering|Material|SetMaterial _light1 0 "/Game/Models/EMF/Material.Material")
        (CallFunction|ResetState)))))

(event EventPickUp
  (bind _body (Variables|Default|GetBody))
  ;[1 1 1] Pick Up
  (Physics|SetSimulatePhysics _body false) ; Disable Physics so it can sit in a single point in the world
  (bind _asbp_first_person_character (Utilities|Casting|CastToBP_FirstPersonCharacter (Game|GetPlayerCharacter 0)))
  (Transformation|AttachComponentToComponent _body (Variables|/Game/Blueprints/Character/BP_FirstPersonCharacter.BP_FirstPersonCharacter_C|GetItemHoldPoint _asbp_first_person_character) "None" "KeepRelative" "KeepRelative" "KeepWorld" true) ; Make the Torch a child of the Item Hold Point
  (Transformation|SetWorldLocation _body (Transformation|GetWorldLocation (Variables|/Game/Blueprints/Character/BP_FirstPersonCharacter.BP_FirstPersonCharacter_C|GetItemHoldPoint _asbp_first_person_character)) false false) ; Set the World Location of the Torch to the World Location of the Item Hold Point
  (Transformation|SetRelativeRotation _body "-90.000000,180.000000,15.000000" false false) ; Set the Relative Rotation so it sits nicely in hand
  (Variables|Default|SetIsHeld true))

(event EventDrop
  ;[1 1 1] Drop
  (Transformation|DetachFromActor "KeepWorld" "KeepRelative" "KeepWorld")
  (Physics|SetSimulatePhysics (Variables|Default|GetBody) true)
  (Physics|AddImpulse (Variables|Default|GetBody) (* (Math|Vector|GetForwardVector (Variables|Default|GetForward)) 2.5e+02) "None" true)
  (Variables|Default|SetIsHeld false))

(fn ConstructionScript)

(fn ChangeState
  (params (EMFLevel :type Integer))
  (if (Variables|Default|GetIsOn)
    (Development|PrintString (Utilities|String|ToString(Integer) EMFLevel))
    (if (>= EMFLevel 2)
      (Rendering|Material|SetMaterial (Variables|Default|GetLight2) 0 "/Game/Models/EMF/Material_002.Material_002")
      (if (>= EMFLevel 3)
        (Rendering|Material|SetMaterial (Variables|Default|GetLight3) 0 "/Game/Models/EMF/Material_003.Material_003")
        (if (>= EMFLevel 4)
          (Rendering|Material|SetMaterial (Variables|Default|GetLight4) 0 "/Game/Models/EMF/Material_004.Material_004")
          (if (>= EMFLevel 5)
            (Rendering|Material|SetMaterial (Variables|Default|GetLight5) 0 "/Game/Models/EMF/Material_005.Material_005")))))))

(fn ResetState
  (bind _light1 (Variables|Default|GetLight1))
  (if (Variables|Default|GetIsOn)
    (Rendering|Material|SetMaterial _light1 0 "/Game/Models/EMF/Material_001.Material_001")
    (else
      (Rendering|Material|SetMaterial _light1 0 "/Game/Models/EMF/Material.Material")))
  (Rendering|Material|SetMaterial (Variables|Default|GetLight2) 0 "/Game/Models/EMF/Material.Material")
  (Rendering|Material|SetMaterial (Variables|Default|GetLight3) 0 "/Game/Models/EMF/Material.Material")
  (Rendering|Material|SetMaterial (Variables|Default|GetLight4) 0 "/Game/Models/EMF/Material.Material")
  (Rendering|Material|SetMaterial (Variables|Default|GetLight5) 0 "/Game/Models/EMF/Material.Material"))