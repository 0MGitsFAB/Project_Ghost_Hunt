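; Handheld lighter item that the player can pick up, drop and toggle open or closed.
; Pickup disables physics and attaches the body to the first-person character's ItemHoldPoint; drop detaches it, restores physics and throws it forward with an impulse.
; Interact flips IsOn and calls ToggleLid, which snaps the lid between two rotations without any flame or light logic.
; GetIsHeld is a stub that always returns false.
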(event EventBeginPlay
  (Transformation|SetRelativeRotation (Variables|Default|GetLid) "0, 0,-145.000000" false false)
  (Variables|Default|SetIsOn false))

(event EventInteract
  (bind _output_get (Variables|Default|SetIsOn (not (Variables|Default|GetIsOn))))
  (CallFunction|ToggleLid _output_get))

(event EventDrop
  ;[1 1 1] Drop
  (Transformation|DetachFromActor "KeepWorld" "KeepRelative" "KeepWorld")
  (Physics|SetSimulatePhysics (Variables|Default|GetBodyBase) true)
  (Rendering|SetActorHiddenInGame false)
  (Physics|AddImpulse (Variables|Default|GetBodyBase) (* (Math|Vector|GetForwardVector (Variables|Default|GetForward)) 1e+03) "None" false))

(event EventPickUp
  (bind _bodybase (Variables|Default|GetBodyBase))
  ;[1 1 1] Pick Up
  (Physics|SetSimulatePhysics _bodybase false) ; Disable Physics so it can sit in a single point in the world
  (bind _asbp_first_person_character (Utilities|Casting|CastToBP_FirstPersonCharacter (Game|GetPlayerCharacter 0)))
  (Transformation|AttachComponentToComponent _bodybase (Variables|/Game/Blueprints/Character/BP_FirstPersonCharacter.BP_FirstPersonCharacter_C|GetItemHoldPoint _asbp_first_person_character) "None" "KeepRelative" "KeepRelative" "KeepWorld" true) ; Make the Torch a child of the Item Hold Point
  (Transformation|SetWorldLocation _bodybase (Transformation|GetWorldLocation (Variables|/Game/Blueprints/Character/BP_FirstPersonCharacter.BP_FirstPersonCharacter_C|GetItemHoldPoint _asbp_first_person_character)) false false) ; Set the World Location of the Torch to the World Location of the Item Hold Point
  (Transformation|SetRelativeRotation _bodybase "0,0.000000, 0" false false) ; Set the Relative Rotation so it sits nicely in hand
)

(fn ConstructionScript)

(fn ToggleLid
  (params (IsOn :type Boolean))
  (bind _lid (Variables|Default|GetLid))
  (if IsOn
    (Transformation|SetRelativeRotation _lid "0, 0,0.000000" false false)
    (else
      (Transformation|SetRelativeRotation _lid "0, 0,-145.000000" false false))))

(fn GetIsHeld
  (return false))