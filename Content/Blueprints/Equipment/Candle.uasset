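; Candle equipment Blueprint that lights itself on BeginPlay, then starts fading out after a fixed delay.
; LightCandle and UnlightCandle are self-calling events that use short Delays to step the PointLight intensity up quickly and down more slowly.
; The Lit flag ends each loop once intensity passes its upper or lower threshold.
; Each step prints an intensity value for debugging.
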(event Custom|Light%20Candle
  ;[1 1 1] Lighting
  (Rendering|Components|Light|SetIntensity (Variables|Default|GetPointLight) (+ (Variables|Default|GetCandleIntesity) 1e+01))
  (Variables|Default|SetCandleIntesity (+ (Variables|Default|GetCandleIntesity) 1e+01))
  (if (> (+ (Variables|Default|GetCandleIntesity) 1e+01) 5e+02)
    (Variables|Default|Setlit true))
  (Development|PrintString (Utilities|String|ToString(Float) (+ (Variables|Default|GetCandleIntesity) 1e+01)))
  (Utilities|FlowControl|Delay 0.1)
  (if (not (Variables|Default|Getlit))
    (CallFunction|LightCandle)))

(event Custom|Unlight%20Candle
  ;[1 1 1] Fading
  (Rendering|Components|Light|SetIntensity (Variables|Default|GetPointLight) (- (Variables|Default|GetCandleIntesity) 5.0))
  (Variables|Default|SetCandleIntesity (- (Variables|Default|GetCandleIntesity) 5.0))
  (if (<= (- (Variables|Default|GetCandleIntesity) 5.0) 0.0)
    (Variables|Default|Setlit false))
  (Development|PrintString (Utilities|String|ToString(Float) (- (Variables|Default|GetCandleIntesity) 5.0)))
  (Utilities|FlowControl|Delay 0.5)
  (if (Variables|Default|Getlit)
    (CallFunction|UnlightCandle)))

(event EventBeginPlay
  (CallFunction|LightCandle)
  (Utilities|FlowControl|Delay 2e+01)
  (CallFunction|UnlightCandle))

(event Collision|EventActorBeginOverlap
  (params (OtherActor :type Actor%20Object%20Reference)))

(event EventTick
  (params (DeltaSeconds :type Float%20%28single-precision%29)))

(fn ConstructionScript)