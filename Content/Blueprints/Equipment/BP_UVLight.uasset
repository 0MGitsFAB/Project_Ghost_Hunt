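; BP_UVLight is a handheld UV torch that the player can pick up, drop and switch on or off.
; PickUp disables physics and attaches the Torch to the first-person character's ItemHoldPoint, snapping its location and resetting its relative rotation.
; Drop detaches it, restores physics and tosses it with an impulse along the Forward component's direction.
; Use toggles the UVLight's visibility, gated by the IsHeld flag that PickUp and Drop maintain.
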(event EventUse
  ;[1 1 1] Interact
  (if (Variables|Default|GetIsHeld)
    (Rendering|ToggleVisibility (Variables|Default|GetUVLight) false)))

(event EventPickUp
  (bind _torch (Variables|Default|GetTorch))
  ;[1 1 1] Pick Up
  (Physics|SetSimulatePhysics _torch false) ; Disable Physics so it can sit in a single point in the world
  (bind _asbp_first_person_character (Utilities|Casting|CastToBP_FirstPersonCharacter (Game|GetPlayerCharacter 0)))
  (Transformation|AttachComponentToComponent _torch (Variables|/Game/Blueprints/Character/BP_FirstPersonCharacter.BP_FirstPersonCharacter_C|GetItemHoldPoint _asbp_first_person_character) "None" "KeepRelative" "KeepRelative" "KeepWorld" true) ; Make the Torch a child of the Item Hold Point
  (Transformation|SetWorldLocation _torch (Transformation|GetWorldLocation (Variables|/Game/Blueprints/Character/BP_FirstPersonCharacter.BP_FirstPersonCharacter_C|GetItemHoldPoint _asbp_first_person_character)) false false) ; Set the World Location of the Torch to the World Location of the Item Hold Point
  (Transformation|SetRelativeRotation _torch "0, 0, 0" false false) ; Set the Relative Rotation so it sits nicely in hand
  (Variables|Default|SetIsHeld true))

(event EventDrop
  ;[1 1 1] Drop
  (Transformation|DetachFromActor "KeepWorld" "KeepRelative" "KeepWorld")
  (Physics|SetSimulatePhysics (Variables|Default|GetTorch) true)
  (Physics|AddImpulse (Variables|Default|GetTorch) (* (Math|Vector|GetForwardVector (Variables|Default|GetForward)) 2.5e+02) "None" true)
  (Variables|Default|SetIsHeld false))

(fn ConstructionScript)