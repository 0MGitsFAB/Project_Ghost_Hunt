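; DragDoorv1 is a door Actor prototype meant to be dragged open and closed while holding LMB and looking at it.
; Tick snaps Door yaw to OpenAngle or ClosedAngle when past either limit, but its rotation step is zero.
; The camera line trace that detects the door, flag resets and TurnRate-driven movement sit in graphs that never run.
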(event EventBeginPlay
  ;[1 1 1] Enable Input
  (Input|EnableInput (Game|GetPlayerController 0)))

(event EventTick
  (params (DeltaSeconds :type Float%20%28single-precision%29))
  (bind _door (Variables|Default|GetDoor))
  (bind _openangle (Variables|Default|GetOpenAngle))
  (bind _closedangle (Variables|Default|GetClosedAngle))
  (bind _door_2 (Variables|Default|GetDoor))
  (bind _returnvalue (Transformation|GetWorldRotation _door))
  (bind _returnvalue_2 (> (.yaw _returnvalue) _openangle))
  (if (Variables|Default|GetIsHoldingLMB)
    (if (Variables|Default|GetIsLookingAtDoor)
      (if _returnvalue_2
        (Variables|Default|SetAngleSurpassed true :!label _label)
        (if _returnvalue_2
          (Transformation|SetRelativeRotation _door_2 (Math|Rotator|MakeRotator 0.0 0.0 _openangle) false false)
          (else
            (Transformation|SetRelativeRotation _door_2 (Math|Rotator|MakeRotator 0.0 0.0 _closedangle) false false)))
        (Variables|Default|SetAngleSurpassed false)
        (if (== (.yaw _returnvalue) _openangle)
          (if true
            (if (not (Variables|Default|GetAngleSurpassed)) :!label _label_2
              (Transformation|AddLocalRotation (Variables|Default|GetDoor) (Math|Rotator|MakeRotator 0.0 0.0 (* 0.0 (Variables|Default|GetSensitivity))) false false)))
          (elif (== (.yaw _returnvalue) _closedangle)
            (if true
              (goto _label_2))))
        (elif (< (.yaw _returnvalue) _closedangle)
          (goto _label)
          (else
            (goto _label_2)))))))

(event Input|ActionEvents|InputActionDoorDrag
  (params (Key :type Key%20Structure :default "None"))
  ;[1 1 1] Check The Player Is Looking At The Door
)

(fn ConstructionScript)