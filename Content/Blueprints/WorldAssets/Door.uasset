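; Door world asset that flags whether it can move when something begins overlapping its Cube component.
; The overlap sets IsMoveable true only if the other component's object type is GameTraceChannel1 and the Cube's world yaw lies within ClosedAngle and OpenAngle, inclusive.
; Any other overlap clears the flag.
; The graph does not rotate the door itself, and the construction script is empty.
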(event OnComponentBeginOverlap(Cube)
  (params (OverlappedComponent :type Primitive%20Component%20Object%20Reference) (OtherActor :type Actor%20Object%20Reference) (OtherComp :type Primitive%20Component%20Object%20Reference) (OtherBodyIndex :type Integer) (bFromSweep :type Boolean) (SweepResult :type Hit%20Result%20Structure%20%28by%20ref%29))
  (if (Utilities|Enum|Equal(Enum) "ECC_GameTraceChannel1" (Collision|GetCollisionObjectType OtherComp))
    (if (<= (.yaw (Transformation|GetWorldRotation (Variables|Default|GetCube))) (Variables|Default|GetOpenAngle))
      (if (>= (.yaw (Transformation|GetWorldRotation (Variables|Default|GetCube))) (Variables|Default|GetClosedAngle))
        (Variables|Default|SetIsMoveable true)
        (else
          (Variables|Default|SetIsMoveable false :!label _label)))
      (else
        (goto _label)))
    (else
      (goto _label))))

(fn ConstructionScript)