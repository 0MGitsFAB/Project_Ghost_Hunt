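; LevelDatbaseActor is a world actor that generates a random temperature reading for a level.
; On BeginPlay it calls UpdateTemperature with state 1, which prints a random value between MinTemp and MaxTemp.
; States 2 and 3 first raise both bounds by one or two StepUpModifier steps, permanently shifting the range, then print.
; The value is only printed, never stored.
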(event EventBeginPlay
  (CallFunction|UpdateTemperature 1))

(fn ConstructionScript)

(fn UpdateTemperature
  (params (TempState :type Integer))
  (if (== TempState 1)
    (Development|PrintString (Utilities|String|ToString(Float) (Math|Random|RandomFloatinRange (LocalVariables|GetMinTemp) (LocalVariables|GetMaxTemp))))
    (elif (== TempState 2)
      (bind _output_get (LocalVariables|SetMinTemp (+ (LocalVariables|GetMinTemp) (LocalVariables|GetStepUpModifier))))
      (bind _output_get_2 (LocalVariables|SetMaxTemp (+ (LocalVariables|GetMaxTemp) (LocalVariables|GetStepUpModifier))))
      (Development|PrintString (Utilities|String|ToString(Float) (Math|Random|RandomFloatinRange _output_get _output_get_2)))
      (elif (== TempState 3)
        (bind _output_get_3 (LocalVariables|SetMinTemp (+ (LocalVariables|GetMinTemp) (* (LocalVariables|GetStepUpModifier) 2.0))))
        (bind _output_get_4 (LocalVariables|SetMaxTemp (+ (LocalVariables|GetMaxTemp) (* (LocalVariables|GetStepUpModifier) 2.0))))
        (Development|PrintString (Utilities|String|ToString(Float) (Math|Random|RandomFloatinRange _output_get_3 _output_get_4)))))))